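; BP_Enemy is an enemy actor that damages the top-down player character on contact and is destroyed when it dies.
; Overlapping its EnemyCollision component with a BP_TopDownCharacter applies PlayerDamage to that character's health component.
; Its own BPHealthComponent reports death through an event bound at BeginPlay, which destroys the actor.
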(event `self.ReceiveBeginPlay`
  (add `/Game/Gameplay/Components/BP_HealthComponent.OnDeath` (`self.BP_HealthComponent`) (delegate `EnemyDeath`)))

(event `EnemyDeath`
  (`self.K2_DestroyActor`))

(event `self.EnemyCollision.OnComponentBeginOverlap`
  (params (OverlappedComponent :type "PrimitiveComponent Object Reference") (OtherActor :type "Actor Object Reference") (OtherComp :type "PrimitiveComponent Object Reference") (OtherBodyIndex :type Integer) (bFromSweep :type Boolean) (SweepResult :type "HitResult Structure (by ref)"))
  (bind _asbp_top_down_character (cast `/Game/TopDown/Blueprints/BP_TopDownCharacter` OtherActor))
  (`/Game/Gameplay/Components/BP_HealthComponent.TakeDamage` (`/Game/TopDown/Blueprints/BP_TopDownCharacter.BP_HealthComponent` _asbp_top_down_character) (`self.PlayerDamage `)))

(fn `UserConstructionScript`)