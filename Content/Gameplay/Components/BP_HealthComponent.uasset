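; Health component that tracks an actor's health and signals death.
; TakeDamage and Heal adjust Health, clamped between zero and MaxHealth.
; TakeDamage calls OnDeath whenever the result is zero, with no guard against repeat calls on further damage.
; BeginPlay and Tick are unused.
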(fn `Heal`
  (params (HealAmount :type "Float (double-precision)"))
  (set `self.Health` (`KismetMathLibrary.FClamp` (+ HealAmount (`self.Health`)) 0.0 (`self.MaxHealth`))))

(fn `TakeDamage`
  (params (Damage :type "Float (double-precision)"))
  (set `self.Health` (`KismetMathLibrary.FClamp` (- (`self.Health`) Damage) 0.0 (`self.MaxHealth`)))
  (if (<= (`self.Health`) 0.0)
    (`self.OnDeath`)))